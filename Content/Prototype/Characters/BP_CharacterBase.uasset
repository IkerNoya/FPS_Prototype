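; BP_CharacterBase is a prototype base character that links to the player HUD and manages walk speed changes.
; On BeginPlay it caches BP_PlayerHUD from its player controller, and ToggleInventory forwards to that HUD when valid.
; HandleSpeedChange plays a timeline that repeatedly lerps MaxWalkSpeed from the current max speed toward the requested one, scaling alpha by delta time and VelocityChangeSpeed for eased transitions.
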(event `self.ReceiveBeginPlay`
  (bind _playercontroller (`self.GetPlayerController`))
  (`/Engine/EditorBlueprintResources/StandardMacros.IsValid` _playercontroller
    (:`Is Valid`
      (bind _asbp_player_hud (cast `/Game/Prototype/Blueprints/UI/BP_PlayerHUD` (`PlayerController.GetHUD` _playercontroller)))
      (set `self.HUD` _asbp_player_hud))))

(event `self.ToggleInventory`
  (`/Engine/EditorBlueprintResources/StandardMacros.IsValid` (`self.HUD`)
    (:`Is Valid`
      (`/Game/Prototype/Blueprints/UI/BP_PlayerHUD.ToggleInventory` (`self.HUD`)))))

(event `self.HandleSpeedChange`
  (params (NewSpeed :type "Float (single-precision)"))
  (bind (_direction _alpha) (`Timeline|SpeedChange` :!via `PlayFromStart`)
    (:`Update`
      (set `CharacterMovementComponent.MaxWalkSpeed` (`KismetMathLibrary.Lerp` (`MovementComponent.GetMaxSpeed` (`self.CharacterMovement`)) NewSpeed (* _alpha (`GameplayStatics.GetWorldDeltaSeconds`) (`self.VelocityChangeSpeed`))) (`self.CharacterMovement`)))))

(fn `UserConstructionScript`)